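; BPTempPlatform is a Paper2D stage platform that disappears after the player touches it, then reappears.
; A hit on its Box from BPPlayer calls TimeToEat, which plays the non-looping flipbook after a short delay.
; When the flipbook finishes, the sprite hides and the Box ignores a custom collision channel.
; After another brief delay, it rewinds the flipbook, shows the sprite and blocks that channel again.
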(event OnComponentHit(Box)
  (params (HitComponent :type Primitive%20Component%20Object%20Reference) (OtherActor :type Actor%20Object%20Reference) (OtherComp :type Primitive%20Component%20Object%20Reference) (NormalImpulse :type Vector :default "0, 0, 0") (Hit :type Hit%20Result%20Structure%20%28by%20ref%29))
  (Utilities|Casting|CastToBPPlayer OtherActor)
  (CallFunction|TimetoEat))

(event OnFinishedPlaying(PaperFlipbook)
  (bind _paperflipbook (Variables|Default|GetPaperFlipbook))
  (bind _paperflipbook_2 (Variables|Default|GetPaperFlipbook))
  (Audio|Components|Audio|Stop _paperflipbook)
  (Rendering|SetVisibility _paperflipbook false false)
  (Collision|SetCollisionResponsetoChannel (Variables|Default|GetBox) "ECC_GameTraceChannel1" "ECR_Ignore")
  (Utilities|FlowControl|Delay 0.5)
  (Components|Timeline|PlayfromStart _paperflipbook_2)
  (Audio|Components|Audio|Stop _paperflipbook_2)
  (Rendering|SetVisibility _paperflipbook_2 true false)
  (Collision|SetCollisionResponsetoChannel (Variables|Default|GetBox) "ECC_GameTraceChannel1" "ECR_Block"))

(event Custom|TimeToEat
  (Utilities|FlowControl|Delay 0.4)
  (Audio|Components|Audio|Play (Variables|Default|GetPaperFlipbook)))

(event EventBeginPlay
  (bind _paperflipbook (Variables|Default|GetPaperFlipbook))
  (Audio|Components|Audio|Stop _paperflipbook)
  (Components|Timeline|SetLooping _paperflipbook false))

(event Collision|EventActorBeginOverlap
  (params (OtherActor :type Actor%20Object%20Reference)))

(event EventTick
  (params (DeltaSeconds :type Float%20%28single-precision%29)))

(fn ConstructionScript)