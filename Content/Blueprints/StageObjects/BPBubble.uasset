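; BPBubble is a stage object with character movement that carries its Box component along a spline and destroys itself at the end.
; On BeginPlay it switches character movement to Flying mode.
; Each Tick advances spline time by delta time scaled by Speed and places the Box at that world location using constant-velocity sampling, without sweeping.
; The overlap and hit events are empty.
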(event OnComponentHit(Box)
  (params (HitComponent :type Primitive%20Component%20Object%20Reference) (OtherActor :type Actor%20Object%20Reference) (OtherComp :type Primitive%20Component%20Object%20Reference) (NormalImpulse :type Vector :default "0, 0, 0") (Hit :type Hit%20Result%20Structure%20%28by%20ref%29)))

(event EventBeginPlay
  (Pawn|Components|CharacterMovement|SetMovementMode (Variables|Character|GetCharacterMovement) "MOVE_Flying" 0))

(event Collision|EventActorBeginOverlap
  (params (OtherActor :type Actor%20Object%20Reference)))

(event EventTick
  (params (DeltaSeconds :type Float%20%28single-precision%29))
  (bind _output_get (Variables|Default|SetTimeOnSpline (+ (Variables|Default|GetTimeOnSpline) (* DeltaSeconds (Variables|Default|GetSpeed)))))
  (Transformation|SetWorldLocation (Variables|Default|GetBox) (Spline|GetLocationatTime (Variables|Default|GetSpline) _output_get "World" true) false false)
  (if (>= (Variables|Default|GetTimeOnSpline) (Variables|/Script/Engine.SplineComponent|GetDuration (Variables|Default|GetSpline)))
    (Actor|DestroyActor)))

(fn ConstructionScript)