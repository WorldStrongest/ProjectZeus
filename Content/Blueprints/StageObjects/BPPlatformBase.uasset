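; Base platform stage object that fits its Box component to the horizontal span between GroundLeft and GroundRight.
; The construction script derives a whole rung count from that span and RungOffset, then scales the Box's X extent by it.
; It also repositions the Box along X using the count and BoxBaseXExtent, keeping Y and Z.
; The event graph contains no active logic.
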(event EventBeginPlay)

(event Collision|EventActorBeginOverlap
  (params (OtherActor :type Actor%20Object%20Reference)))

(event EventTick
  (params (DeltaSeconds :type Float%20%28single-precision%29)))

(fn ConstructionScript
  (bind _groundleft (Variables|Default|GetGroundLeft))
  (bind _groundright (Variables|Default|GetGroundRight))
  (bind _rungoffset (Variables|Default|GetRungOffset))
  (bind _box (Variables|Default|GetBox))
  (bind _box_2 (Variables|Default|GetBox))
  (bind _boxbasexextent (Variables|Default|GetBoxBaseXExtent))
  (bind _returnvalue (- _groundright _groundleft))
  (bind _relativelocation (Variables|/Script/Engine.SceneComponent|GetRelativeLocation _box))
  (bind _x (Math|Vector|BreakVector _returnvalue))
  (bind (_x_2 _y _z) (Math|Vector|BreakVector _relativelocation))
  (bind _returnvalue_2 (/ _x _rungoffset))
  (bind _returnvalue_3 (Math|Float|Truncate _returnvalue_2))
  (|CallParentFunction)
  (Components|Box|SetBoxExtent _box_2 (* (Math|Vector|MakeVector (Math|Conversions|ToFloat(Integer) (+ _returnvalue_3 1)) 1.0 1.0) (Variables|/Script/Engine.BoxComponent|GetBoxExtent _box)) true)
  (Transformation|SetRelativeLocation _box_2 (Math|Vector|MakeVector (+ (* (- _returnvalue_3 1) _boxbasexextent) _boxbasexextent) _y _z) false false))