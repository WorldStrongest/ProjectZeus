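; BPLinePlatform is a stage platform that moves in a straight line to an end point once the player enters its trigger.
; BeginPlay caches the platform and EndPoint world locations and sets the PlatformMove timeline rate to the inverse of Playrate.
; An overlap on PlayerTouch by a BPPlayer plays the timeline forward, lerping the platform between those locations without sweep.
; The graph has no return movement.
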(event OnComponentBeginOverlap(PlayerTouch)
  (params (OverlappedComponent :type Primitive%20Component%20Object%20Reference) (OtherActor :type Actor%20Object%20Reference) (OtherComp :type Primitive%20Component%20Object%20Reference) (OtherBodyIndex :type Integer) (bFromSweep :type Boolean) (SweepResult :type Hit%20Result%20Structure%20%28by%20ref%29))
  (Utilities|Casting|CastToBPPlayer OtherActor)
  (bind _alpha (Timeline|PlatformMove Play)
    (:Update
      (Transformation|SetWorldLocation (Variables|Default|GetPlatform) (Math|Vector|Lerp(Vector) (Variables|Default|GetStartLocation) (Variables|Default|GetEndLocation) _alpha) false false))))

(event EventBeginPlay
  (Variables|Default|SetStartLocation (Transformation|GetWorldLocation (Variables|Default|GetPlatform)))
  (Variables|Default|SetEndLocation (Transformation|GetWorldLocation (Variables|Default|GetEndPoint)))
  (Components|Timeline|SetPlayRate (Variables|Default|GetPlatformMove) (/ 1.0 (Variables|Default|GetPlayrate))))

(fn ConstructionScript)