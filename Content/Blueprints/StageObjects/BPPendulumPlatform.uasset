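; BPPendulumPlatform is a stage object that moves a Box component back and forth along a Spline, like a pendulum platform.
; Each Tick advances or rewinds a time value by Speed, depending on a Reverse flag, and places the box at that constant-velocity point in world space without sweeping.
; Reverse flips when the time reaches the spline's Duration or drops to zero.
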(event EventBeginPlay)

(event Collision|EventActorBeginOverlap
  (params (OtherActor :type Actor%20Object%20Reference)))

(event EventTick
  (params (DeltaSeconds :type Float%20%28single-precision%29))
  (bind _speed (Variables|Default|GetSpeed))
  (bind _returnvalue (* DeltaSeconds _speed))
  (bind _output_get (Variables|Default|SetTimeOnSpline (Math|Float|SelectFloat (- (Variables|Default|GetTimeOnSpline) _returnvalue) (+ (Variables|Default|GetTimeOnSpline) _returnvalue) (Variables|Default|GetbReverse))))
  (Transformation|SetWorldLocation (Variables|Default|GetBox) (Spline|GetLocationatTime (Variables|Default|GetSpline) _output_get "World" true) false false)
  (if (and (not (Variables|Default|GetbReverse)) (>= (Variables|Default|GetTimeOnSpline) (Variables|/Script/Engine.SplineComponent|GetDuration (Variables|Default|GetSpline))))
    (Variables|Default|SetbReverse true)
    (elif (and (<= (Variables|Default|GetTimeOnSpline) 0.0) (Variables|Default|GetbReverse))
      (Variables|Default|SetbReverse false))))

(fn ConstructionScript)