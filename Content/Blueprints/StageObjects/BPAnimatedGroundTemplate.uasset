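; Template Blueprint for an animated stage ground piece, built from a row of Paper2D flipbooks.
; The construction script derives the tile count from the X distance between GroundLeft and GroundRight divided by RungOffset.
; It adds a flipbook component at each step along local X, cycling through the GroundPartFlipbook array by wrapping FlipbookIndex.
; The event graph holds only disabled placeholder events, so all logic runs at construction.
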(event EventBeginPlay)

(event Collision|EventActorBeginOverlap
  (params (OtherActor :type Actor%20Object%20Reference)))

(event EventTick
  (params (DeltaSeconds :type Float%20%28single-precision%29)))

(fn ConstructionScript
  (bind _rungoffset (Variables|Default|GetRungOffset))
  (for _index (range 0 (Math|Float|Truncate (/ (.X (Math|Vector|BreakVector (- (Variables|Default|GetGroundRight) (Variables|Default|GetGroundLeft)))) _rungoffset)))
    (bind _returnvalue (AddComponent|AddPaperFlipbookComponent false (Math|Transform|MakeTransform (Math|Transform|TransformLocation (Math|Transform|MakeTransform "0, 0, 0") (Math|Vector|MakeVector (* _index _rungoffset) 0.0 0.0)))))
    (Sprite|SetFlipbook _returnvalue (Utilities|Array|Get(acopy) (Variables|Default|GetGroundPartFlipbook) (Variables|Default|GetFlipbookIndex)))
    (bind _result (Math|Integer|IncrementInt (Variables|Default|GetFlipbookIndex))
      (:%20%20
        (Variables|Default|SetFlipbookIndex (Math|Integer|%(Integer) _result (Utilities|Array|Length (Variables|Default|GetGroundPartFlipbook))))))))