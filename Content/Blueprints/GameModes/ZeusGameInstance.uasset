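; Game instance that applies saved display settings and background music volume at startup.
; On Init it loads GameUserSettings, reapplies the resolution and fullscreen mode, then overrides the music sound class in the BGM sound mix with VolumeBGM and pushes that mix.
; ChangeVolume repeats the same override and push to apply the current VolumeBGM value on demand.
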(event EventInit
  (Utilities|FlowControl|Sequence
    (:then_0
      (bind _returnvalue (Settings|GetGameUserSettings))
      (Class|GameUserSettings|LoadSettings _returnvalue false)
      (Class|GameUserSettings|SetScreenResolution _returnvalue (Class|GameUserSettings|GetScreenResolution _returnvalue))
      (Class|GameUserSettings|SetFullscreenMode _returnvalue (Class|GameUserSettings|GetFullscreenMode _returnvalue))
      (Class|GameUserSettings|ApplyResolutionSettings _returnvalue false))
    (:then_1
      (Audio|SetSoundMixClassOverride "/Game/Audio/Mixes/SM_BGM.SM_BGM" "/Game/Audio/Classes/SC_Music.SC_Music" (Variables|Default|GetVolumeBGM) 1.0 1.0 true)
      (Audio|PushSoundMixModifier "/Game/Audio/Mixes/SM_BGM.SM_BGM"))))

(event EventShutdown)

(fn ChangeVolume
  (Audio|SetSoundMixClassOverride "/Game/Audio/Mixes/SM_BGM.SM_BGM" "/Game/Audio/Classes/SC_Music.SC_Music" (Variables|Default|GetVolumeBGM) 1.0 1.0 true)
  (Audio|PushSoundMixModifier "/Game/Audio/Mixes/SM_BGM.SM_BGM"))