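; Enemy Blueprint with a sprite that handles taking damage by either dying or flashing.
; TakeDamage destroys the actor when HealthCurrent minus the damage is zero or less, though it never stores the reduced health.
; Otherwise it runs a looping timer on Blink for about a second, briefly hiding and re-showing EnemySprite.
; BeginPlay, Tick, overlap and capsule hit events are empty.
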(event OnComponentHit(CapsuleComponent)
  (params (HitComponent :type Primitive%20Component%20Object%20Reference) (OtherActor :type Actor%20Object%20Reference) (OtherComp :type Primitive%20Component%20Object%20Reference) (NormalImpulse :type Vector :default "0, 0, 0") (Hit :type Hit%20Result%20Structure%20%28by%20ref%29)))

(event Custom|Blink
  (bind _enemysprite (Variables|Default|GetEnemySprite))
  (Development|SetHiddeninGame _enemysprite true false)
  (Utilities|FlowControl|Delay 0.1)
  (Development|SetHiddeninGame _enemysprite false false))

(event Custom|TakeDamage
  (params (DamageVal :type Float%20%28single-precision%29))
  (if (<= (- (Variables|Default|GetHealthCurrent) DamageVal) 0.0)
    (Actor|DestroyActor)
    (else
      (Utilities|Time|SetTimerbyFunctionName 0 "Blink" 0.1 true)
      (Utilities|FlowControl|Delay 1.0)
      (Utilities|Time|ClearTimerbyFunctionName 0 "Blink"))))

(event EventBeginPlay)

(event Collision|EventActorBeginOverlap
  (params (OtherActor :type Actor%20Object%20Reference)))

(event EventTick
  (params (DeltaSeconds :type Float%20%28single-precision%29)))

(fn ConstructionScript)