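; BPTest is a Paper2D enemy character that walks back and forth along the world X axis.
; Every tick, the Direction event yaws the sprite to face its heading and adds movement input that way, based on IsMovingRight.
; Any capsule hit toggles IsMovingRight, turning it around, with no filtering of what was struck.
; Actor overlaps only forward to the parent class.
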(event OnComponentHit(CapsuleComponent)
  (params (HitComponent :type Primitive%20Component%20Object%20Reference) (OtherActor :type Actor%20Object%20Reference) (OtherComp :type Primitive%20Component%20Object%20Reference) (NormalImpulse :type Vector :default "0, 0, 0") (Hit :type Hit%20Result%20Structure%20%28by%20ref%29))
  (Variables|Default|SetIsMovingRight (not (Variables|Default|GetIsMovingRight))))

(event Custom|Direction
  (Transformation|SetRelativeRotation (Variables|Default|GetPaperSprite) (Math|Rotator|MakeRotator 0.0 0.0 (Math|Float|SelectFloat 0.0 1.8e+02 (Variables|Default|GetIsMovingRight))) false false)
  (Pawn|Input|AddMovementInput (Math|Vector|SelectVector "1.000000, 0, 0" "-1.000000, 0, 0" (Variables|Default|GetIsMovingRight)) 1.0 false))

(event EventBeginPlay
  ;[1 1 1] BeginPlay
)

(event Collision|EventActorBeginOverlap
  (params (OtherActor :type Actor%20Object%20Reference))
  (|CallParentFunction OtherActor))

(event EventTick
  (params (DeltaSeconds :type Float%20%28single-precision%29))
  ;[1 1 1] Tick
  (CallFunction|Direction))

(fn ConstructionScript
  (|CallParentFunction))