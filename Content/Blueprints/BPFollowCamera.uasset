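; BPFollowCamera is a follow-camera actor that tracks the first player pawn along the world X and Z axes while holding its own Y position.
; Each Tick, if the pawn is valid, it adds WorldOffset to the pawn's location and eases the actor toward that point with VInterpTo at a fixed speed.
; The move is not swept, and rotation is never changed.
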(event EventBeginPlay)

(event Collision|EventActorBeginOverlap
  (params (OtherActor :type Actor%20Object%20Reference)))

(event EventTick
  (params (DeltaSeconds :type Float%20%28single-precision%29))
  (bind _returnvalue (Game|Player|GetPlayerPawn 0))
  (bind _returnvalue_2 (Transformation|GetActorLocation))
  (bind _worldoffset (Variables|Default|GetWorldOffset))
  (bind _returnvalue_3 (Transformation|GetActorLocation _returnvalue))
  (bind _returnvalue_4 (+ _returnvalue_3 _worldoffset))
  (bind (_x _y _z) (Math|Vector|BreakVector _returnvalue_4))
  (Utilities|IsValid _returnvalue
    (:Is%20Valid
      (Transformation|SetActorLocation (Math|Interpolation|VInterpTo _returnvalue_2 (Math|Vector|MakeVector _x (.Y (Math|Vector|BreakVector _returnvalue_2)) _z) DeltaSeconds 1e+01) false false))))

(fn ConstructionScript)