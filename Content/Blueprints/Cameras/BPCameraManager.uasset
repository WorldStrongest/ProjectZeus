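; Level camera manager that spawns a BPFollowCamera and switches its mode from trigger boxes.
; On BeginPlay it hands the camera a reference to itself, then binds overlap events on its attached TriggerBox actors.
; Entering a box sets the camera to a follow-all mode, and leaving sets another mode.
; A MoveTo handler exists but is never bound, as the name-based selection for it is unused.
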(event Custom|CameraMoveTo
  (params (OverlappedActor :type Actor%20Object%20Reference) (OtherActor :type Actor%20Object%20Reference))
  (Default|Moveto (Variables|Default|GetCameraRef)))

(event Custom|CameraFollowAll
  (params (OverlappedActor :type Actor%20Object%20Reference) (OtherActor :type Actor%20Object%20Reference))
  (Variables|/Game/Blueprints/Cameras/BPFollowCamera.BPFollowCamera_C|SetCameraMode (Variables|Default|GetCameraRef) "NewEnumerator4"))

(event Custom|CameraEndFollowAll
  (params (OverlappedActor :type Actor%20Object%20Reference) (OtherActor :type Actor%20Object%20Reference))
  (Variables|/Game/Blueprints/Cameras/BPFollowCamera.BPFollowCamera_C|SetCameraMode (Variables|Default|GetCameraRef) "NewEnumerator0"))

(event EventBeginPlay
  (bind _returnvalue (Game|SpawnActorfromClass "/Game/Blueprints/Cameras/BPFollowCamera.BPFollowCamera_C" (Math|Transform|MakeTransform "0, 0, 0") "Undefined" 0 0))
  (bind _output_get (Variables|Default|SetCameraRef _returnvalue))
  (Variables|/Game/Blueprints/Cameras/BPFollowCamera.BPFollowCamera_C|SetManager _output_get self)
  (bind _output_get_2 (Variables|Default|SetBoxTriggers (Actor|GetAttachedActors)))
  (for _array_element _output_get_2
    (bind _astrigger_box (Utilities|Casting|CastToTriggerBox _array_element))
    (Collision|BindEventtoOnActorBeginOverlap _astrigger_box (delegate Custom|CameraFollowAll))
    (Collision|BindEventtoOnActorEndOverlap _astrigger_box (delegate Custom|CameraEndFollowAll))))

(event Collision|EventActorBeginOverlap
  (params (OtherActor :type Actor%20Object%20Reference)))

(event EventTick
  (params (DeltaSeconds :type Float%20%28single-precision%29)))

(fn ConstructionScript)