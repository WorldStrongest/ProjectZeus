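; Side-scrolling pixel-art camera that follows the player pawn with a world offset.
; BeginPlay positions it at the player after a short delay; Tick interpolates at constant speed and snaps to the pixel grid.
; Modes follow X only, also follow Z (held while grounded and still horizontally), move to a stored height, or glide to a locked location.
; Ortho-width scaling, player dispatcher bindings and automatic return from MoveTo are disconnected.
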(event Custom|MoveToPlayer
  (Variables|Default|SetCameraMode "NewEnumerator1")
  (Variables|Default|SetZLocation (.Z (Math|Vector|BreakVector (+ (Transformation|GetActorLocation (Game|Player|GetPlayerPawn 0)) (Variables|Default|GetWorldOffset))))))

(event Custom|FollowAllMode
  (Variables|Default|SetCameraMode "NewEnumerator4"))

(event Custom|StopFollowAllMode
  (Variables|Default|SetCameraMode "NewEnumerator0"))

(event EventBeginPlay
  (Transformation|SetActorLocation (Math|Vector|MakeVector 0.0 (Variables|Default|GetZLocation) 0.0) false false)
  (Utilities|FlowControl|Delay 0.2)
  (Transformation|SetActorLocation (+ (Transformation|GetActorLocation (Game|Player|GetPlayerPawn 0)) (Variables|Default|GetWorldOffset)) false false))

(event Collision|EventActorBeginOverlap
  (params (OtherActor :type Actor%20Object%20Reference)))

(event EventTick
  (params (DeltaSeconds :type Float%20%28single-precision%29))
  (bind _returnvalue (Transformation|GetActorLocation))
  (bind _returnvalue_2 (Game|Player|GetPlayerPawn 0))
  (bind _returnvalue_3 (Game|Player|GetPlayerPawn 0))
  (bind _cameramode (Variables|Default|GetCameraMode))
  (bind _worldoffset (Variables|Default|GetWorldOffset))
  (bind _returnvalue_4 (Pawn|GetMovementComponent _returnvalue_2))
  (bind _returnvalue_5 (Transformation|GetActorLocation _returnvalue_3))
  (bind (_x _y _z) (Math|Vector|BreakVector _returnvalue))
  (bind _returnvalue_6 (Utilities|Enum|Equal(Enum) _cameramode "NewEnumerator0"))
  (bind _returnvalue_7 (Utilities|Enum|Equal(Enum) _cameramode "NewEnumerator4"))
  (bind _returnvalue_8 (AI|Components|NavMovement|IsMovingonGround _returnvalue_4))
  (bind _returnvalue_9 (+ _returnvalue_5 _worldoffset))
  (bind _velocity (Variables|/Script/Engine.MovementComponent|GetVelocity _returnvalue_4))
  (bind _x_2 (Math|Vector|BreakVector _velocity))
  (bind (_x_3 _y_2 _z_2) (Math|Vector|BreakVector _returnvalue_9))
  (bind _returnvalue_10 (Math|Float|NearlyEqual(Float) _x_2 0.0 1e-06))
  (bind _returnvalue_11 (Math|Boolean|ANDBoolean _returnvalue_7 _returnvalue_8 _returnvalue_10))
  (bind _returnvalue_12 (or _returnvalue_6 _returnvalue_11))
  (bind _returnvalue_13 (Math|Float|SelectFloat _z _z_2 _returnvalue_12))
  (bind _returnvalue_14 (Math|Vector|MakeVector _x_3 _y _returnvalue_13))
  (bind _returnvalue_15 (Math|Interpolation|VInterptoConstant _returnvalue _returnvalue_14 DeltaSeconds 1e+03))
  (bind (_x_4 _y_3 _z_3) (Math|Vector|BreakVector _returnvalue_15))
  (Utilities|IsValid _returnvalue_3
    (:Is%20Valid
      (switch Utilities|FlowControl|Switch|SwitchonCameraMode_Enum (Variables|Default|GetCameraMode)
        (:NewEnumerator0
          (bind _outvector (CallFunction|SnapVectortoGrid (Math|Vector|SelectVector _returnvalue_15 (Math|Vector|MakeVector _x_4 _y_3 (Math|Interpolation|FInterptoConstant _z (Variables|Default|GetZLocation) (Utilities|Time|GetWorldDeltaSeconds) 1e+03)) (or (Utilities|Enum|Equal(Enum) _cameramode "NewEnumerator0") (Utilities|Enum|Equal(Enum) _cameramode "NewEnumerator4"))) 1.0 :!label _label))
          (Transformation|SetActorLocation _outvector false false))
        (:NewEnumerator1
          (goto _label))
        (:NewEnumerator3
          (Components|MoveComponentTo (Variables|Default|GetSceneComponent) (Variables|Default|GetTargetLocation) "0, 0, 0" false false (Variables|Default|GetOverTime) false))
        (:NewEnumerator4
          (goto _label))))))

(fn ConstructionScript)

(fn GetPixelArtScale
  (params (InViewPortSize :type Vector%202D%20Structure))
  (return (Math|Conversions|ToFloat(Integer) (Math|Integer|Max(Integer) (Math|Float|Round (/ (.X (Math|Vector2D|BreakVector2D InViewPortSize)) (.X (Math|Vector2D|BreakVector2D (Variables|Default|GetReferenceResolution))))) 1))))

(fn Moveto
  (Variables|Default|SetCameraMode "NewEnumerator1")
  (Variables|Default|SetZLocation (.Z (Math|Vector|BreakVector (+ (Transformation|GetActorLocation (Game|Player|GetPlayerPawn 0)) (Variables|Default|GetWorldOffset))))))

(fn LockonLocation
  (params (TargetLocation :type Vector) (OverTime :type Float%20%28single-precision%29))
  (Variables|Default|SetTargetLocation TargetLocation)
  (Variables|Default|SetOverTime OverTime)
  (Variables|Default|SetCameraMode "NewEnumerator3"))