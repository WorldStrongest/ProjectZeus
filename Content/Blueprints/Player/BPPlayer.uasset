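; BPPlayer is the player character for a 2D flipbook side-scrolling platformer, handling movement, combat and damage.
; A CurrentState switch gates input and picks animations for running, crouching, double jumps, climbing, wall clinging and wall jumps.
; Attack and dive-kick boxes toggle collision to damage BPEnemy, with dive-kick hits bouncing the player, while enemy overlaps cause knockback and blinking.
; Collision-response switching enables pass-through platforms; dash logic is disconnected.
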(event OnComponentHit(CapsuleComponent)
  (params (HitComponent :type Primitive%20Component%20Object%20Reference) (OtherActor :type Actor%20Object%20Reference) (OtherComp :type Primitive%20Component%20Object%20Reference) (NormalImpulse :type Vector :default "0, 0, 0") (Hit :type Hit%20Result%20Structure%20%28by%20ref%29))
  ;[1 1 1] Collision
  (if (and (Utilities|Enum|NotEqual(Enum) (Variables|Default|GetCurrentState) "NewEnumerator4") (Utilities|Enum|Equal(Enum) (Collision|GetCollisionObjectType OtherComp) "ECC_GameTraceChannel3"))
    (if (< (.Z (Math|Vector|BreakVector (Variables|/Script/Engine.MovementComponent|GetVelocity (Variables|Character|GetCharacterMovement)))) 0.0)
      (CallFunction|SetWallClinging true))))

(event OnComponentBeginOverlap(AttackBox)
  (params (OverlappedComponent :type Primitive%20Component%20Object%20Reference) (OtherActor :type Actor%20Object%20Reference) (OtherComp :type Primitive%20Component%20Object%20Reference) (OtherBodyIndex :type Integer) (bFromSweep :type Boolean) (SweepResult :type Hit%20Result%20Structure%20%28by%20ref%29))
  ;[1 1 1] GroundAttack
  (bind _asbpenemy (Utilities|Casting|CastToBPEnemy OtherActor))
  (Default|TakeDamage _asbpenemy 0.0))

(event OnComponentBeginOverlap(DiveKickBox)
  (params (OverlappedComponent :type Primitive%20Component%20Object%20Reference) (OtherActor :type Actor%20Object%20Reference) (OtherComp :type Primitive%20Component%20Object%20Reference) (OtherBodyIndex :type Integer) (bFromSweep :type Boolean) (SweepResult :type Hit%20Result%20Structure%20%28by%20ref%29))
  (bind _charactermovement (Variables|Character|GetCharacterMovement))
  ;[1 1 1] DiveKick Atack
  (bind _asbpenemy (Utilities|Casting|CastToBPEnemy OtherActor))
  (Default|TakeDamage _asbpenemy 0.0)
  (Variables|/Script/Engine.MovementComponent|SetVelocity _charactermovement (Math|Vector|MakeVector (.X (Math|Vector|BreakVector (Variables|/Script/Engine.MovementComponent|GetVelocity _charactermovement))) 0.0 0.0))
  (Character|LaunchCharacter (Math|Vector|SelectVector (Variables|Default|GetDiveKickHeldHitVelocity) (Variables|Default|GetDiveKickHitVelocity) (Variables|Default|GetbAttackPressed)) false false)
  (Collision|SetCollisionResponsetoChannel (Variables|Default|GetDiveKickBox) "ECC_GameTraceChannel4" "ECR_Ignore")
  (Variables|Default|SetDoubleJumpAvailable true)
  (Variables|Default|SetDashAvailable true)
  (Variables|Default|SetCurrentState "NewEnumerator8")
  (CallFunction|UpdateAnimation))

(event OnComponentBeginOverlap(CapsuleComponent)
  (params (OverlappedComponent :type Primitive%20Component%20Object%20Reference) (OtherActor :type Actor%20Object%20Reference) (OtherComp :type Primitive%20Component%20Object%20Reference) (OtherBodyIndex :type Integer) (bFromSweep :type Boolean) (SweepResult :type Hit%20Result%20Structure%20%28by%20ref%29))
  (bind _currentstate (Variables|Default|GetCurrentState))
  ;[1 1 1] Collision
  (switch Utilities|FlowControl|Switch|SwitchonECollisionChannel (Collision|GetCollisionObjectType OtherComp)
    (:ECC_GameTraceChannel6
      (Variables|Default|SetbInsidePlatform true))
    (:ECC_GameTraceChannel7
      (if (not (or (Utilities|Enum|Equal(Enum) _currentstate "NewEnumerator9") (Utilities|Enum|Equal(Enum) _currentstate "NewEnumerator6")))
        (bind _asbpenemy (Utilities|Casting|CastToBPEnemy OtherActor))
        (CallFunction|TakeDamage (Variables|/Game/Blueprints/Enemies/BPEnemy.BPEnemy_C|GetDamageVal _asbpenemy))))))

(event OnComponentEndOverlap(CapsuleComponent)
  (params (OverlappedComponent :type Primitive%20Component%20Object%20Reference) (OtherActor :type Actor%20Object%20Reference) (OtherComp :type Primitive%20Component%20Object%20Reference) (OtherBodyIndex :type Integer))
  ;[1 1 1] Collision
  (if (Utilities|Enum|Equal(Enum) (Collision|GetCollisionObjectType OtherComp) "ECC_GameTraceChannel6")
    (Variables|Default|SetbInsidePlatform false)))

(event Custom|Blink
  (bind _sprite (Variables|Default|GetSprite))
  ;[1 1 1] Handle Damage
  (Development|SetHiddeninGame _sprite true false)
  (Utilities|FlowControl|Delay 0.1)
  (Development|SetHiddeninGame _sprite false false))

(event Custom|ResetGravity
  (bind _charactermovement (Variables|Character|GetCharacterMovement))
  ;[1 1 1] Handle Dash
  (if (Utilities|Enum|Equal(Enum) (Variables|/Script/Engine.CharacterMovementComponent|GetMovementMode _charactermovement) "MOVE_Flying")
    (Pawn|Components|CharacterMovement|SetMovementMode _charactermovement "MOVE_Falling" 0)))

(event Custom|UpdateAnimation
  (bind _sprite (Variables|Default|GetSprite))
  ;[1 1 1] Handle Animation
  (switch Utilities|FlowControl|Switch|SwitchonPlayerState_Enum (Variables|Default|GetCurrentState)
    (:NewEnumerator0
      (Sprite|SetFlipbook (Variables|Default|GetSprite) (select (> (Math|Vector|VectorLength (Transformation|GetVelocity)) 0.0) "/Game/Sprites/Characters/PlayerEnlarged300/Run/Protag_Run.Protag_Run" "/Game/Sprites/Characters/PlayerEnlarged300/Idle/Protag_Idle.Protag_Idle") :!label _label))
    (:NewEnumerator1
      (Sprite|SetFlipbook _sprite "/Game/Sprites/Characters/PlayerEnlarged300/Attack/Protag_Attack.Protag_Attack"))
    (:NewEnumerator4
      (Sprite|SetFlipbook _sprite "/Game/Sprites/Characters/PlayerEnlarged300/Divekick/Protag_Divekick.Protag_Divekick"))
    (:NewEnumerator7
      (goto _label))
    (:NewEnumerator8
      (Sprite|SetFlipbook _sprite "/Game/Sprites/Characters/PlayerEnlarged300/Jump/Protag_Jump.Protag_Jump"))
    (:NewEnumerator12
      (Sprite|SetFlipbook _sprite "/Game/Sprites/Characters/PlayerEnlarged300/Crouch/Protag_Crouch.Protag_Crouch"))))

(event Custom|TakeDamage
  (params (DamageVal :type Float%20%28single-precision%29))
  (bind _knockback (Variables|Default|GetKnockback))
  ;[1 1 1] Handle Damage
  (Variables|/Script/Engine.MovementComponent|SetVelocity (Variables|Character|GetCharacterMovement) "0, 0, 0")
  (bind _output_get (Variables|Default|SetHealthCurrent (- (Variables|Default|GetHealthCurrent) DamageVal)))
  (Development|PrintText (Utilities|Text|ToText(Float) _output_get "HalfToEven"))
  (if (<= _output_get 0.0)
    (Variables|Default|SetCurrentState "NewEnumerator6")
    (else
      (Variables|Default|SetCurrentState "NewEnumerator9")
      (Physics|AddForce (Variables|Character|GetCharacterMovement) (Math|Vector|MakeVector (* (Variables|Default|GetFacing) _knockback) 0.0 _knockback))
      (Utilities|Time|SetTimerbyFunctionName 0 "Blink" 0.1 true)
      (Utilities|FlowControl|Delay 0.6)
      (Utilities|Time|ClearTimerbyFunctionName 0 "Blink")
      (if (AI|Components|NavMovement|IsMovingonGround (Variables|Character|GetCharacterMovement))
        (Variables|Default|SetCurrentState "NewEnumerator0")
        (else
          (Variables|Default|SetCurrentState "NewEnumerator8"))))))

(event EventOnLanded
  (params (Hit :type Hit%20Result%20Structure%20%28by%20ref%29))
  ;[1 1 1] Handle Jump
  (Default|CallCameraMovetoDispatcher)
  (if (not (Utilities|Enum|Equal(Enum) (Variables|Default|GetCurrentState) "NewEnumerator9"))
    (if (Game|Player|IsInputKeyDown (Game|GetPlayerController 0) (Variables|Default|GetCrouchKeyRef))
      (Variables|Default|SetCurrentState "NewEnumerator12")
      (Character|Crouch)
      (CallFunction|UpdateAnimation)
      (else
        (Variables|Default|SetCurrentState "NewEnumerator0")))
    (Collision|SetCollisionResponsetoChannel (Variables|Default|GetDiveKickBox) "ECC_GameTraceChannel4" "ECR_Ignore")
    (Variables|Default|SetDoubleJumpAvailable true)
    (Variables|Default|SetDashAvailable true)))

(event EventTick
  (params (DeltaSeconds :type Float%20%28single-precision%29))
  (bind _charactermovement (Variables|Character|GetCharacterMovement))
  (bind _capsulecomponent (Variables|Collision|GetCapsuleComponent))
  ;[1 1 1] Tick - Updates animation
  (switch Utilities|FlowControl|Switch|SwitchonPlayerState_Enum (Variables|Default|GetCurrentState)
    (:NewEnumerator0
      (if (AI|Components|NavMovement|IsMovingonGround _charactermovement) :!label _label
        (Variables|Default|SetCurrentState "NewEnumerator0")
        (else
          (Variables|Default|SetCurrentState "NewEnumerator8"))))
    (:NewEnumerator4
      (if (or (Variables|Default|GetbInsidePlatform) (>= (.Z (Math|Vector|BreakVector (Variables|/Script/Engine.MovementComponent|GetVelocity _charactermovement))) 0.1)) :!label _label_2
        (Collision|SetCollisionResponsetoChannel _capsulecomponent "ECC_GameTraceChannel6" "ECR_Overlap")
        (else
          (Collision|SetCollisionResponsetoChannel _capsulecomponent "ECC_GameTraceChannel6" "ECR_Block"))))
    (:NewEnumerator8
      (Utilities|FlowControl|Sequence
        (:then_0
          (goto _label_2))
        (:then_1
          (goto _label))))))

(event EventBeginPlay
  ;[1 1 1] Initialize
  (Class|ActorComponent|SetIsReplicated (Variables|Default|GetSprite) true)
  (Variables|/Script/Engine.PhysicsVolume|SetFluidFriction (Class|MovementComponent|GetPhysicsVolume (Variables|Character|GetCharacterMovement)) 0.0))

(event Input|ActionEvents|InputActionDash
  (params (Key :type Key%20Structure))
  ;[1 1 1] Handle Dash
)

(event Input|ActionEvents|InputActionAttack
  (params (Key :type Key%20Structure))
  ;[1 1 1] Handle Attack
  (:Pressed
    (Variables|Default|SetbAttackPressed true)
    (switch Utilities|FlowControl|Switch|SwitchonPlayerState_Enum (Variables|Default|GetCurrentState)
      (:NewEnumerator0
        (Variables|Default|SetCurrentState "NewEnumerator1")
        (Collision|SetCollisionResponsetoChannel (Variables|Default|GetAttackBox) "ECC_GameTraceChannel4" "ECR_Overlap")
        (CallFunction|UpdateAnimation)
        (Utilities|FlowControl|Delay 0.1)
        (if (Utilities|Enum|Equal(Enum) (Variables|Default|GetCurrentState) "NewEnumerator1")
          (Variables|Default|SetCurrentState "NewEnumerator0")
          (Collision|SetCollisionResponsetoChannel (Variables|Default|GetAttackBox) "ECC_GameTraceChannel4" "ECR_Ignore")))
      (:NewEnumerator8
        (Variables|Default|SetCurrentState "NewEnumerator4")
        (Collision|SetCollisionResponsetoChannel (Variables|Default|GetDiveKickBox) "ECC_GameTraceChannel4" "ECR_Overlap")
        (CallFunction|UpdateAnimation))))
  (:Released
    (Variables|Default|SetbAttackPressed false)))

(event Input|ActionEvents|InputActionCrouch
  (params (Key :type Key%20Structure))
  ;[1 1 1] Handle movement
  (:Pressed
    (Variables|Default|SetCrouchKeyRef Key)
    (if (Utilities|Enum|Equal(Enum) (Variables|Default|GetCurrentState) "NewEnumerator0")
      (Variables|Default|SetCurrentState "NewEnumerator12")
      (Character|Crouch)
      (CallFunction|UpdateAnimation :!label _label)))
  (:Released
    (if (Utilities|Enum|Equal(Enum) (Variables|Default|GetCurrentState) "NewEnumerator12")
      (Variables|Default|SetCurrentState "NewEnumerator0")
      (Character|UnCrouch)
      (goto _label))))

(event Input|ActionEvents|InputActionJump
  (params (Key :type Key%20Structure))
  (bind _returnvalue (Game|GetPlayerController 0))
  (bind _charactermovement (Variables|Character|GetCharacterMovement))
  ;[1 1 1] Handle Jump
  (:Pressed
    (switch Utilities|FlowControl|Switch|SwitchonPlayerState_Enum (Variables|Default|GetCurrentState)
      (:NewEnumerator0
        (bind _isonplatform (CallFunction|ChecktoFallThroughPlatform :!label _label))
        (if _isonplatform
          (Collision|SetCollisionResponsetoChannel (Variables|Collision|GetCapsuleComponent) "ECC_GameTraceChannel6" "ECR_Overlap")
          (Variables|Default|SetbInsidePlatform true)
          (else
            (Character|Jump :!label _label_2)))
        (Variables|Default|SetCurrentState "NewEnumerator8" :!label _label_3))
      (:NewEnumerator1
        (Collision|SetCollisionResponsetoChannel (Variables|Default|GetAttackBox) "ECC_GameTraceChannel4" "ECR_Ignore")
        (goto _label_2))
      (:NewEnumerator7
        (if (!= (Input|AxisValues|GetMoveRight) 0.0)
          (CallFunction|SetNotClimbing)
          (Character|LaunchCharacter (Math|Vector|MakeVector 0.0 0.0 (Variables|Default|GetDoubleJumpZVelocity)) false false :!label _label_4)
          (goto _label_3)))
      (:NewEnumerator8
        (if (Variables|Default|GetDoubleJumpAvailable)
          (Variables|Default|SetDoubleJumpAvailable false)
          (Variables|/Script/Engine.MovementComponent|SetVelocity _charactermovement (Math|Vector|MakeVector (.X (Math|Vector|BreakVector (Variables|/Script/Engine.MovementComponent|GetVelocity _charactermovement))) 0.0 0.0))
          (goto _label_4)))
      (:NewEnumerator11
        (Character|LaunchCharacter (Math|Vector|MakeVector (* (Variables|Default|GetFacing) 2.5e+02) 0.0 (Variables|Default|GetDoubleJumpZVelocity)) false false)
        (Variables|Default|SetCurrentState "NewEnumerator8")
        (Input|SetIgnoreMoveInput _returnvalue true)
        (Utilities|FlowControl|Delay 0.3)
        (Input|ResetIgnoreMoveInput _returnvalue))
      (:NewEnumerator12
        (Character|UnCrouch)
        (goto _label))))
  (:Released
    (Character|StopJumping)))

(event Input|AxisEvents|InputAxisMoveUp
  (params (AxisValue :type Float%20%28single-precision%29))
  ;[1 1 1] Handle movement
  (if (!= AxisValue 0.0)
    (switch Utilities|FlowControl|Switch|SwitchonPlayerState_Enum (Variables|Default|GetCurrentState)
      (:NewEnumerator0
        (if (and (Variables|Default|GetbClimbable) (> AxisValue 0.0)) :!label _label
          (CallFunction|SetClimbing)))
      (:NewEnumerator7
        (Transformation|AddActorLocalOffset (Math|Vector|MakeVector 0.0 0.0 (* AxisValue (Variables|Default|GetClimbSpeed))) true false :!label _label_2)
        (CallFunction|UpdateAnimation))
      (:NewEnumerator8
        (goto _label))
      (:NewEnumerator11
        (if (< AxisValue 0.0)
          (goto _label_2))))))

(event Input|AxisEvents|InputAxisMoveRight
  (params (AxisValue :type Float%20%28single-precision%29))
  ;[1 1 1] Handle movement
  (if (not (Class|Pawn|IsMoveInputIgnored))
    (switch Utilities|FlowControl|Switch|SwitchonPlayerState_Enum (Variables|Default|GetCurrentState)
      (:NewEnumerator0
        _)
      (:NewEnumerator4
        _)
      (:NewEnumerator8
        _))
    (Pawn|Input|AddMovementInput "1.000000, 0, 0" AxisValue false)
    (CallFunction|UpdateAnimation)
    (Math|Float|CompareFloat AxisValue 0.0
      (:>
        (Pawn|SetControlRotation (Pawn|GetController) (Math|Rotator|MakeRotator 0.0 0.0 0.0))
        (Variables|Default|SetFacing -1))
      (:<
        (Pawn|SetControlRotation (Pawn|GetController) (Math|Rotator|MakeRotator 0.0 0.0 1.8e+02))
        (Variables|Default|SetFacing 1)))))

(event Input|KeyboardEvents|1
  (params (Key :type Key%20Structure))
  (bind _knockback (Variables|Default|GetKnockback))
  ;[1 1 1] Handle Damage
  (:Pressed
    (Variables|/Script/Engine.MovementComponent|SetVelocity (Variables|Character|GetCharacterMovement) "0, 0, 0")
    (bind _output_get (Variables|Default|SetHealthCurrent (- (Variables|Default|GetHealthCurrent) (stale Custom|TakeDamage DamageVal))))
    (Development|PrintText (Utilities|Text|ToText(Float) _output_get "HalfToEven"))
    (if (<= _output_get 0.0)
      (Variables|Default|SetCurrentState "NewEnumerator6")
      (else
        (Variables|Default|SetCurrentState "NewEnumerator9")
        (Physics|AddForce (Variables|Character|GetCharacterMovement) (Math|Vector|MakeVector (* (Variables|Default|GetFacing) _knockback) 0.0 _knockback))
        (Utilities|Time|SetTimerbyFunctionName 0 "Blink" 0.1 true)
        (Utilities|FlowControl|Delay 0.6)
        (Utilities|Time|ClearTimerbyFunctionName 0 "Blink")
        (if (AI|Components|NavMovement|IsMovingonGround (Variables|Character|GetCharacterMovement))
          (Variables|Default|SetCurrentState "NewEnumerator0")
          (else
            (Variables|Default|SetCurrentState "NewEnumerator8")))))))

(fn ConstructionScript)

(fn SetNotClimbing
  (Variables|Default|SetbClimbable false)
  (CallFunction|ResetGravity)
  (if (Utilities|Enum|Equal(Enum) (Variables|Default|GetCurrentState) "NewEnumerator7")
    (if (AI|Components|NavMovement|IsMovingonGround (Variables|Character|GetCharacterMovement))
      (Variables|Default|SetCurrentState "NewEnumerator0")
      (else
        (Variables|Default|SetCurrentState "NewEnumerator8")))
    (Default|CallCameraStopFollowAllDispatcher)))

(fn SetWallClinging
  (params (bWallClinging :type Boolean))
  (bind _charactermovement (Variables|Character|GetCharacterMovement))
  (bind _charactermovement_2 (Variables|Character|GetCharacterMovement))
  (if bWallClinging
    (Variables|Default|SetCurrentState "NewEnumerator11")
    (Variables|/Script/Engine.MovementComponent|SetVelocity _charactermovement "0, 0, 0")
    (Pawn|Components|CharacterMovement|SetMovementMode _charactermovement "MOVE_Flying" 0)
    (Default|CallCameraFollowAllDispatcher)
    (else
      (if (Utilities|Enum|Equal(Enum) (Variables|Default|GetCurrentState) "NewEnumerator9")
        (Pawn|Components|CharacterMovement|SetMovementMode _charactermovement_2 "MOVE_Falling" 0 :!label _label)
        (elif (AI|Components|NavMovement|IsMovingonGround (Variables|Character|GetCharacterMovement))
          (Variables|Default|SetCurrentState "NewEnumerator0")
          (Pawn|Components|CharacterMovement|SetMovementMode _charactermovement_2 "MOVE_Walking" 0)
          (else
            (Variables|Default|SetCurrentState "NewEnumerator8")
            (goto _label))))
      (Default|CallCameraStopFollowAllDispatcher)))
  (CallFunction|UpdateAnimation))

(fn SetClimbing
  (bind _charactermovement (Variables|Character|GetCharacterMovement))
  (Variables|Default|SetCurrentState "NewEnumerator7")
  (Variables|/Script/Engine.MovementComponent|SetVelocity _charactermovement (Math|Vector|MakeVector 0.0 0.0 0.0)) ; 0 out velocity so we don't slide around
  (Pawn|Components|CharacterMovement|SetMovementMode _charactermovement "MOVE_Flying" 0)
  (Default|CallCameraFollowAllDispatcher)
  (CallFunction|UpdateAnimation))

(fn ChecktoFallThroughPlatform
  (bind _returnvalue (Transformation|GetActorLocation))
  (bind _returnvalue_2 (Collision|LineTraceForObjects _returnvalue (- _returnvalue "0, 0,40.000000") (Utilities|Array|MakeArray "ObjectTypeQuery12") false 0 "None"))
  (return (and _returnvalue_2 (< (Input|AxisValues|GetMoveUp) 0.0))))

(fn GetCrouchOffset
  (return (- (Variables|/Script/Engine.CapsuleComponent|GetCapsuleHalfHeight (Variables|Collision|GetCapsuleComponent)) (Variables|/Script/Engine.CharacterMovementComponent|GetCrouchedHalfHeight (Variables|Character|GetCharacterMovement)))))