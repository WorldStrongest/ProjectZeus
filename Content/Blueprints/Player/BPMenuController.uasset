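; BPMenuController is a player controller for the main menu, driven by input actions with the mouse cursor hidden.
; On BeginPlay it creates the MainMenuSwitcher widget, adds it to the viewport and focuses it in Game and UI input mode.
; MenuUp and MenuDown presses move through the widget, and the Attack action doubles as confirm by calling its DoMenuAction.
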(event EventBeginPlay
  (Variables|Default|SetbShowMouseCursor false)
  (bind _returnvalue (UserInterface|CreateWidget "/Game/Blueprints/UI/MainMenuSwitcher.MainMenuSwitcher_C" self))
  (UserInterface|Viewport|AddtoViewport _returnvalue 0)
  (Input|SetInputModeGameandUI self _returnvalue "DoNotLock" true)
  (Variables|Default|SetMainMenuSwitcherRef _returnvalue))

(event EventTick
  (params (DeltaSeconds :type Float%20%28single-precision%29)))

(event Input|ActionEvents|InputActionMenuDown
  (params (Key :type Key%20Structure))
  (:Pressed
    (Default|MoveDown (Variables|Default|GetMainMenuSwitcherRef))))

(event Input|ActionEvents|InputActionMenuUp
  (params (Key :type Key%20Structure))
  (:Pressed
    (Default|MoveUp (Variables|Default|GetMainMenuSwitcherRef))))

(event Input|ActionEvents|InputActionAttack
  (params (Key :type Key%20Structure))
  (:Pressed
    (Default|DoMenuAction (Variables|Default|GetMainMenuSwitcherRef))))

(fn ConstructionScript)