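; Player-controlled map cursor that moves over points of interest and opens their levels.
; Sets flying movement on BeginPlay, then input axes offset it directly along X and Z by Speed, without sweep or delta-time scaling.
; MoveClamp projects each proposed position to screen space and zeroes movement past the viewport edges, with a margin on the horizontal sides.
; Overlap events track the current BPPOI, and Attack opens its Level.
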(event EventBeginPlay
  ;[1 1 1] Initialize
  (Utilities|FlowControl|Sequence
    (:then_0
      (Class|ActorComponent|SetIsReplicated (Variables|Default|GetSprite) true))
    (:then_1
      (Pawn|Components|CharacterMovement|SetMovementMode (Variables|Character|GetCharacterMovement) "MOVE_Flying" 0))))

(event Collision|EventActorBeginOverlap
  (params (OtherActor :type Actor%20Object%20Reference))
  (bind _asbppoi (Utilities|Casting|CastToBPPOI OtherActor))
  (Variables|Default|SetPOIref _asbppoi))

(event EventTick
  (params (DeltaSeconds :type Float%20%28single-precision%29)))

(event Collision|EventActorEndOverlap
  (params (OtherActor :type Actor%20Object%20Reference))
  (Utilities|Casting|CastToBPPOI OtherActor)
  (Variables|Default|SetPOIref 0))

(event Input|ActionEvents|InputActionAttack
  (params (Key :type Key%20Structure))
  (bind _poiref (Variables|Default|GetPOIref))
  (:Pressed
    (if (Utilities|IsValid _poiref)
      (Game|OpenLevel(byName) (Variables|/Game/Blueprints/StageObjects/BPPOI.BPPOI_C|GetLevel _poiref)))))

(event Input|AxisEvents|InputAxisMoveUp
  (params (AxisValue :type Float%20%28single-precision%29))
  ;[1 1 1] Handle Movement
  (if (!= AxisValue 0.0)
    (bind _newdeltalocation (CallFunction|MoveClamp (Math|Vector|MakeVector 0.0 0.0 (* AxisValue (Variables|Default|GetSpeed)))))
    (Transformation|AddActorWorldOffset _newdeltalocation)))

(event Input|AxisEvents|InputAxisMoveRight
  (params (AxisValue :type Float%20%28single-precision%29))
  ;[1 1 1] Handle Movement
  (if (!= AxisValue 0.0)
    (bind _newdeltalocation (CallFunction|MoveClamp (Math|Vector|MakeVector (* AxisValue (Variables|Default|GetSpeed)) 0.0 0.0)))
    (Transformation|AddActorWorldOffset _newdeltalocation)))

(fn ConstructionScript)

(fn MoveClamp
  (params (DeltaLocation :type Vector))
  (bind _returnvalue (Game|GetPlayerController 0))
  (bind _returnvalue_2 (Transformation|GetActorLocation))
  (bind _returnvalue_3 (Viewport|GetViewportSize))
  (bind (_x _y _z) (Math|Vector|BreakVector DeltaLocation))
  (bind (_x_2 _y_2) (Math|Vector2D|BreakVector2D _returnvalue_3))
  (bind _returnvalue_4 (+ DeltaLocation _returnvalue_2))
  (bind _screenposition (Class|GameplayStatics|ProjectWorldtoScreen _returnvalue _returnvalue_4 false))
  (bind _returnvalue_5 (/ _x_2 2e+01))
  (bind (_x_3 _y_3) (Math|Vector2D|BreakVector2D _screenposition))
  (return (Math|Vector|MakeVector (Math|Float|SelectFloat 0.0 _x (or (>= _x_3 (- _x_2 _returnvalue_5)) (<= _x_3 _returnvalue_5))) 0.0 (Math|Float|SelectFloat 0.0 _z (or (>= _y_3 _y_2) (<= _y_3 0.0))))))