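; Player character Blueprint for a 2D side-scrolling platformer, using a Paper2D sprite that swaps idle and running flipbooks and turns with movement input.
; A state variable gates movement, jump with double jump, and a gravity-free directional air dash; landing restores both air abilities.
; Key 1 triggers test damage, leading to death or a timed hit state with knockback and timer-driven sprite blinking.
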(event Custom|Blink
  (bind _sprite (Variables|Default|GetSprite))
  ;[1 1 1] Handle Damage
  (Development|SetHiddeninGame _sprite true false)
  (Utilities|FlowControl|Delay 0.1)
  (Development|SetHiddeninGame _sprite false false))

(event Custom|UpdateAnimation
  ;[1 1 1] Handle Animation
  (Sprite|SetFlipbook (Variables|Default|GetSprite) (select (> (Math|Vector|VectorLength (Transformation|GetVelocity)) 0.0) "/Game/2DSideScroller/Sprites/RunningAnimation.RunningAnimation" "/Game/2DSideScroller/Sprites/IdleAnimation.IdleAnimation")))

(event EventOnLanded
  (params (Hit :type Hit%20Result%20Structure%20%28by%20ref%29))
  ;[1 1 1] Handle Jump
  (if (not (Utilities|Enum|Equal(Enum) (Variables|Default|GetCurrentState) "NewEnumerator9"))
    (Variables|Default|SetCurrentState "NewEnumerator0")
    (Variables|Default|SetDoubleJumpAvailable true)
    (Variables|Default|SetDashAvailable true)))

(event EventTick
  (params (DeltaSeconds :type Float%20%28single-precision%29))
  ;[1 1 1] Tick - Updates animation
)

(event EventBeginPlay
  (Class|ActorComponent|SetIsReplicated (Variables|Default|GetSprite) true))

(event Input|ActionEvents|InputActionDash
  (params (Key :type Key%20Structure))
  (bind _dashvelocity (Variables|Default|GetDashVelocity))
  (bind _charactermovement (Variables|Character|GetCharacterMovement))
  (bind _charactermovement_2 (Variables|Character|GetCharacterMovement))
  ;[1 1 1] Handle Dash
  (:Pressed
    (if (Variables|Default|GetDashAvailable)
      (switch Utilities|FlowControl|Switch|SwitchonPlayerState_Enum (Variables|Default|GetCurrentState)
        (:NewEnumerator8
          (Variables|Default|SetDashAvailable false)
          (Variables|Default|SetCurrentState "NewEnumerator5")
          (Variables|/Script/Engine.CharacterMovementComponent|SetGravityScale _charactermovement_2 0.0)
          (Variables|/Script/Engine.MovementComponent|SetVelocity _charactermovement_2 "0, 0, 0")
          (Character|LaunchCharacter (Math|Vector|MakeVector (* (Input|AxisValues|GetMoveRight) _dashvelocity) 0.0 (* _dashvelocity (Input|AxisValues|GetMoveUp))) false false)
          (Utilities|FlowControl|Delay 0.35)
          (Variables|/Script/Engine.CharacterMovementComponent|SetGravityScale _charactermovement 2.0)
          (if (Utilities|Enum|NotEqual(Enum) (Variables|Default|GetCurrentState) "NewEnumerator9")
            (Variables|/Script/Engine.MovementComponent|SetVelocity _charactermovement "0, 0, 0")
            (if (not (Utilities|Enum|Equal(Enum) (Variables|Default|GetCurrentState) "NewEnumerator6"))
              (if (AI|Components|NavMovement|IsMovingonGround _charactermovement)
                (Variables|Default|SetCurrentState "NewEnumerator0")
                (else
                  (Variables|Default|SetCurrentState "NewEnumerator8"))))))))))

(event Input|ActionEvents|InputActionJump
  (params (Key :type Key%20Structure))
  (bind _charactermovement (Variables|Character|GetCharacterMovement))
  ;[1 1 1] Handle Jump
  (:Pressed
    (switch Utilities|FlowControl|Switch|SwitchonPlayerState_Enum (Variables|Default|GetCurrentState)
      (:NewEnumerator0
        (Character|Jump :!label _label)
        (Variables|Default|SetCurrentState "NewEnumerator8" :!label _label_2))
      (:NewEnumerator1
        (goto _label))
      (:NewEnumerator4
        (goto _label))
      (:NewEnumerator8
        (if (Variables|Default|GetDoubleJumpAvailable)
          (Variables|Default|SetDoubleJumpAvailable false)
          (Variables|/Script/Engine.MovementComponent|SetVelocity _charactermovement (Math|Vector|MakeVector (.X (Math|Vector|BreakVector (Variables|/Script/Engine.MovementComponent|GetVelocity _charactermovement))) 0.0 0.0))
          (Character|LaunchCharacter (Math|Vector|MakeVector 0.0 0.0 (Variables|Default|GetDoubleJumpZVelocity)) false false)
          (goto _label_2)))))
  (:Released
    (Character|StopJumping)))

(event Input|AxisEvents|InputAxisMoveRight
  (params (AxisValue :type Float%20%28single-precision%29))
  ;[1 1 1] Handle movement
  (switch Utilities|FlowControl|Switch|SwitchonPlayerState_Enum (Variables|Default|GetCurrentState)
    (:NewEnumerator0
      _)
    (:NewEnumerator8
      _))
  (Pawn|Input|AddMovementInput "1.000000, 0, 0" AxisValue false)
  (CallFunction|UpdateAnimation)
  (Math|Float|CompareFloat AxisValue 0.0
    (:>
      (Pawn|SetControlRotation (Pawn|GetController) (Math|Rotator|MakeRotator 0.0 0.0 0.0))
      (Variables|Default|SetFacing -1))
    (:<
      (Pawn|SetControlRotation (Pawn|GetController) (Math|Rotator|MakeRotator 0.0 0.0 1.8e+02))
      (Variables|Default|SetFacing 1))))

(event Input|KeyboardEvents|1
  (params (Key :type Key%20Structure))
  ;[1 1 1] Handle Damage
  (:Pressed
    (bind _output_get (Variables|Default|SetHealthCurrent (- (Variables|Default|GetHealthCurrent) 0.25)))
    (if (<= _output_get 0.0)
      (Variables|Default|SetCurrentState "NewEnumerator6")
      (else
        (Variables|Default|SetCurrentState "NewEnumerator9")
        (Physics|AddForce (Variables|Character|GetCharacterMovement) (Math|Vector|MakeVector (* (Variables|Default|GetFacing) (Variables|Default|GetKnockback)) 0.0 0.0))
        (Utilities|Time|SetTimerbyFunctionName 0 "Blink" 0.1 true)
        (Utilities|FlowControl|Delay 1.0)
        (Utilities|Time|ClearTimerbyFunctionName 0 "Blink")
        (if (AI|Components|NavMovement|IsMovingonGround (Variables|Character|GetCharacterMovement))
          (Variables|Default|SetCurrentState "NewEnumerator0")
          (else
            (Variables|Default|SetCurrentState "NewEnumerator8")))))))

(fn ConstructionScript)