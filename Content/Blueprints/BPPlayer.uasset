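; Paper2D side-scroller player character with running, double jump, climbing, wall cling and jump, punch and dive kick.
; A CurrentState enum gates input, movement and flipbook choice, with Tick and landing resolving standing versus airborne.
; Attacks toggle hitbox collision responses to damage BPEnemy; dive-kick hits bounce the player and restore air moves.
; Damage, also triggered by key 1, applies knockback and timer-driven blinking or death; dash logic exists but is unconnected.
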(event OnComponentHit(CapsuleComponent)
  (params (HitComponent :type Primitive%20Component%20Object%20Reference) (OtherActor :type Actor%20Object%20Reference) (OtherComp :type Primitive%20Component%20Object%20Reference) (NormalImpulse :type Vector :default "0, 0, 0") (Hit :type Hit%20Result%20Structure%20%28by%20ref%29))
  ;[1 1 1] Collision
  (if (and (Utilities|Enum|NotEqual(Enum) (Variables|Default|GetCurrentState) "NewEnumerator4") (Utilities|Enum|Equal(Enum) (Collision|GetCollisionObjectType OtherComp) "ECC_GameTraceChannel3"))
    (if (< (.Z (Math|Vector|BreakVector (Variables|/Script/Engine.MovementComponent|GetVelocity (Variables|Character|GetCharacterMovement)))) 0.0)
      (CallFunction|SetWallClinging true))))

(event OnComponentBeginOverlap(AttackBox)
  (params (OverlappedComponent :type Primitive%20Component%20Object%20Reference) (OtherActor :type Actor%20Object%20Reference) (OtherComp :type Primitive%20Component%20Object%20Reference) (OtherBodyIndex :type Integer) (bFromSweep :type Boolean) (SweepResult :type Hit%20Result%20Structure%20%28by%20ref%29))
  ;[1 1 1] GroundAttack
  (bind _asbpenemy (Utilities|Casting|CastToBPEnemy OtherActor))
  (Default|TakeDamage _asbpenemy 0.0))

(event OnComponentBeginOverlap(DiveKickBox)
  (params (OverlappedComponent :type Primitive%20Component%20Object%20Reference) (OtherActor :type Actor%20Object%20Reference) (OtherComp :type Primitive%20Component%20Object%20Reference) (OtherBodyIndex :type Integer) (bFromSweep :type Boolean) (SweepResult :type Hit%20Result%20Structure%20%28by%20ref%29))
  (bind _charactermovement (Variables|Character|GetCharacterMovement))
  ;[1 1 1] DiveKick Atack
  (bind _asbpenemy (Utilities|Casting|CastToBPEnemy OtherActor))
  (Default|TakeDamage _asbpenemy 0.0)
  (Variables|/Script/Engine.MovementComponent|SetVelocity _charactermovement (Math|Vector|MakeVector (.X (Math|Vector|BreakVector (Variables|/Script/Engine.MovementComponent|GetVelocity _charactermovement))) 0.0 0.0))
  (Character|LaunchCharacter (Math|Vector|SelectVector (Variables|Default|GetDiveKickHeldHitVelocity) (Variables|Default|GetDiveKickHitVelocity) (Variables|Default|GetbAttackPressed)) false false)
  (Collision|SetCollisionResponsetoChannel (Variables|Default|GetDiveKickBox) "ECC_GameTraceChannel4" "ECR_Ignore")
  (Variables|Default|SetDoubleJumpAvailable true)
  (Variables|Default|SetDashAvailable true)
  (Variables|Default|SetCurrentState "NewEnumerator8")
  (CallFunction|UpdateAnimation))

(event Custom|Blink
  (bind _sprite (Variables|Default|GetSprite))
  ;[1 1 1] Handle Damage
  (Development|SetHiddeninGame _sprite true false)
  (Utilities|FlowControl|Delay 0.1)
  (Development|SetHiddeninGame _sprite false false))

(event Custom|ResetGravity
  ;[1 1 1] Handle Dash
  (Pawn|Components|CharacterMovement|SetMovementMode (Variables|Character|GetCharacterMovement) "MOVE_Walking" 0)
  (Variables|/Script/Engine.CharacterMovementComponent|SetGravityScale (Variables|Character|GetCharacterMovement) (Variables|Default|GetDefaultGravity)))

(event Custom|UpdateAnimation
  (bind _sprite (Variables|Default|GetSprite))
  ;[1 1 1] Handle Animation
  (switch Utilities|FlowControl|Switch|SwitchonPlayerState_Enum (Variables|Default|GetCurrentState)
    (:NewEnumerator0
      (Sprite|SetFlipbook (Variables|Default|GetSprite) (select (> (Math|Vector|VectorLength (Transformation|GetVelocity)) 0.0) "/Game/Sprites/Characters/Protag_run.Protag_run" "/Game/Sprites/Characters/Protag_idle.Protag_idle") :!label _label))
    (:NewEnumerator1
      (Sprite|SetFlipbook _sprite "/Game/Sprites/Characters/Protag_Sprite_punch.Protag_Sprite_punch"))
    (:NewEnumerator4
      (Sprite|SetFlipbook _sprite "/Game/Sprites/Characters/Protag_divekick_Flipbook.Protag_divekick_Flipbook"))
    (:NewEnumerator7
      (goto _label))
    (:NewEnumerator8
      (Sprite|SetFlipbook _sprite "/Game/Sprites/Characters/Protag_jump.Protag_jump"))))

(event Custom|TakeDamage
  (params (DamageVal :type Float%20%28single-precision%29))
  ;[1 1 1] Handle Damage
  (Variables|/Script/Engine.MovementComponent|SetVelocity (Variables|Character|GetCharacterMovement) "0, 0, 0")
  (bind _output_get (Variables|Default|SetHealthCurrent (- (Variables|Default|GetHealthCurrent) DamageVal)))
  (if (<= _output_get 0.0)
    (Variables|Default|SetCurrentState "NewEnumerator6")
    (else
      (Variables|Default|SetCurrentState "NewEnumerator9")
      (Physics|AddForce (Variables|Character|GetCharacterMovement) (Math|Vector|MakeVector (* (Variables|Default|GetFacing) (Variables|Default|GetKnockback)) 0.0 0.0))
      (Utilities|Time|SetTimerbyFunctionName 0 "Blink" 0.1 true)
      (Utilities|FlowControl|Delay 1.0)
      (Utilities|Time|ClearTimerbyFunctionName 0 "Blink")
      (if (AI|Components|NavMovement|IsMovingonGround (Variables|Character|GetCharacterMovement))
        (Variables|Default|SetCurrentState "NewEnumerator0")
        (else
          (Variables|Default|SetCurrentState "NewEnumerator8"))))))

(event EventOnLanded
  (params (Hit :type Hit%20Result%20Structure%20%28by%20ref%29))
  ;[1 1 1] Handle Jump
  (if (not (Utilities|Enum|Equal(Enum) (Variables|Default|GetCurrentState) "NewEnumerator9"))
    (Variables|Default|SetCurrentState "NewEnumerator0")
    (Collision|SetCollisionResponsetoChannel (Variables|Default|GetDiveKickBox) "ECC_GameTraceChannel4" "ECR_Ignore")
    (Variables|Default|SetDoubleJumpAvailable true)
    (Variables|Default|SetDashAvailable true)))

(event EventTick
  (params (DeltaSeconds :type Float%20%28single-precision%29))
  ;[1 1 1] Tick - Updates animation
  (switch Utilities|FlowControl|Switch|SwitchonPlayerState_Enum (Variables|Default|GetCurrentState)
    (:NewEnumerator0
      _)
    (:NewEnumerator8
      _))
  (if (AI|Components|NavMovement|IsMovingonGround (Variables|Character|GetCharacterMovement))
    (Variables|Default|SetCurrentState "NewEnumerator0")
    (else
      (Variables|Default|SetCurrentState "NewEnumerator8"))))

(event EventBeginPlay
  ;[1 1 1] Initialize
  (Class|ActorComponent|SetIsReplicated (Variables|Default|GetSprite) true)
  (Variables|/Script/Engine.PhysicsVolume|SetFluidFriction (Class|MovementComponent|GetPhysicsVolume (Variables|Character|GetCharacterMovement)) 0.0))

(event Input|ActionEvents|InputActionDash
  (params (Key :type Key%20Structure))
  ;[1 1 1] Handle Dash
)

(event Input|ActionEvents|InputActionAttack
  (params (Key :type Key%20Structure))
  ;[1 1 1] Handle Attack
  (:Pressed
    (Variables|Default|SetbAttackPressed true)
    (switch Utilities|FlowControl|Switch|SwitchonPlayerState_Enum (Variables|Default|GetCurrentState)
      (:NewEnumerator0
        (Variables|Default|SetCurrentState "NewEnumerator1")
        (Collision|SetCollisionResponsetoChannel (Variables|Default|GetAttackBox) "ECC_GameTraceChannel4" "ECR_Overlap")
        (CallFunction|UpdateAnimation)
        (Utilities|FlowControl|Delay 0.1)
        (if (Utilities|Enum|Equal(Enum) (Variables|Default|GetCurrentState) "NewEnumerator1")
          (Variables|Default|SetCurrentState "NewEnumerator0")
          (Collision|SetCollisionResponsetoChannel (Variables|Default|GetAttackBox) "ECC_GameTraceChannel4" "ECR_Ignore")))
      (:NewEnumerator8
        (Variables|Default|SetCurrentState "NewEnumerator4")
        (Collision|SetCollisionResponsetoChannel (Variables|Default|GetDiveKickBox) "ECC_GameTraceChannel4" "ECR_Overlap")
        (CallFunction|UpdateAnimation))))
  (:Released
    (Variables|Default|SetbAttackPressed false)))

(event Input|ActionEvents|InputActionJump
  (params (Key :type Key%20Structure))
  (bind _returnvalue (Game|GetPlayerController 0))
  (bind _charactermovement (Variables|Character|GetCharacterMovement))
  ;[1 1 1] Handle Jump
  (:Pressed
    (switch Utilities|FlowControl|Switch|SwitchonPlayerState_Enum (Variables|Default|GetCurrentState)
      (:NewEnumerator0
        (Character|Jump :!label _label)
        (Variables|Default|SetCurrentState "NewEnumerator8" :!label _label_2))
      (:NewEnumerator1
        (Collision|SetCollisionResponsetoChannel (Variables|Default|GetAttackBox) "ECC_GameTraceChannel4" "ECR_Ignore")
        (goto _label))
      (:NewEnumerator7
        (Character|LaunchCharacter (Math|Vector|MakeVector 0.0 0.0 (Variables|Default|GetDoubleJumpZVelocity)) false false :!label _label_3)
        (goto _label_2))
      (:NewEnumerator8
        (if (Variables|Default|GetDoubleJumpAvailable)
          (Variables|Default|SetDoubleJumpAvailable false)
          (Variables|/Script/Engine.MovementComponent|SetVelocity _charactermovement (Math|Vector|MakeVector (.X (Math|Vector|BreakVector (Variables|/Script/Engine.MovementComponent|GetVelocity _charactermovement))) 0.0 0.0))
          (goto _label_3)))
      (:NewEnumerator11
        (Character|LaunchCharacter (Math|Vector|MakeVector (* (Variables|Default|GetFacing) 3e+02) 0.0 (Variables|Default|GetDoubleJumpZVelocity)) false false)
        (Variables|Default|SetCurrentState "NewEnumerator8")
        (Input|SetIgnoreMoveInput _returnvalue true)
        (Utilities|FlowControl|Delay 0.2)
        (Input|ResetIgnoreMoveInput _returnvalue))))
  (:Released
    (Character|StopJumping)))

(event Input|AxisEvents|InputAxisMoveUp
  (params (AxisValue :type Float%20%28single-precision%29))
  (bind _charactermovement (Variables|Character|GetCharacterMovement))
  ;[1 1 1] Handle movement
  (if (!= AxisValue 0.0)
    (switch Utilities|FlowControl|Switch|SwitchonPlayerState_Enum (Variables|Default|GetCurrentState)
      (:NewEnumerator0
        (if (Variables|Default|GetbClimbable) :!label _label
          (Variables|Default|SetCurrentState "NewEnumerator7")
          (Variables|/Script/Engine.MovementComponent|SetVelocity _charactermovement (Math|Vector|MakeVector 0.0 0.0 0.0))
          (Pawn|Components|CharacterMovement|SetMovementMode _charactermovement "MOVE_Flying" 0)
          (CallFunction|UpdateAnimation)))
      (:NewEnumerator7
        (Transformation|AddActorLocalOffset (Math|Vector|MakeVector 0.0 0.0 (* AxisValue (Variables|Default|GetClimbSpeed))) false false)
        (CallFunction|UpdateAnimation))
      (:NewEnumerator8
        (goto _label)))))

(event Input|AxisEvents|InputAxisMoveRight
  (params (AxisValue :type Float%20%28single-precision%29))
  ;[1 1 1] Handle movement
  (if (not (Class|Pawn|IsMoveInputIgnored))
    (switch Utilities|FlowControl|Switch|SwitchonPlayerState_Enum (Variables|Default|GetCurrentState)
      (:NewEnumerator0
        _)
      (:NewEnumerator4
        _)
      (:NewEnumerator7
        _)
      (:NewEnumerator8
        _))
    (Pawn|Input|AddMovementInput "1.000000, 0, 0" AxisValue false)
    (CallFunction|UpdateAnimation)
    (Math|Float|CompareFloat AxisValue 0.0
      (:>
        (Pawn|SetControlRotation (Pawn|GetController) (Math|Rotator|MakeRotator 0.0 0.0 0.0))
        (Variables|Default|SetFacing -1))
      (:<
        (Pawn|SetControlRotation (Pawn|GetController) (Math|Rotator|MakeRotator 0.0 0.0 1.8e+02))
        (Variables|Default|SetFacing 1)))))

(event Input|KeyboardEvents|1
  (params (Key :type Key%20Structure))
  ;[1 1 1] Handle Damage
  (:Pressed
    (Variables|/Script/Engine.MovementComponent|SetVelocity (Variables|Character|GetCharacterMovement) "0, 0, 0")
    (bind _output_get (Variables|Default|SetHealthCurrent (- (Variables|Default|GetHealthCurrent) (stale Custom|TakeDamage DamageVal))))
    (if (<= _output_get 0.0)
      (Variables|Default|SetCurrentState "NewEnumerator6")
      (else
        (Variables|Default|SetCurrentState "NewEnumerator9")
        (Physics|AddForce (Variables|Character|GetCharacterMovement) (Math|Vector|MakeVector (* (Variables|Default|GetFacing) (Variables|Default|GetKnockback)) 0.0 0.0))
        (Utilities|Time|SetTimerbyFunctionName 0 "Blink" 0.1 true)
        (Utilities|FlowControl|Delay 1.0)
        (Utilities|Time|ClearTimerbyFunctionName 0 "Blink")
        (if (AI|Components|NavMovement|IsMovingonGround (Variables|Character|GetCharacterMovement))
          (Variables|Default|SetCurrentState "NewEnumerator0")
          (else
            (Variables|Default|SetCurrentState "NewEnumerator8")))))))

(fn ConstructionScript)

(fn SetNotClimbing
  (Variables|Default|SetbClimbable false)
  (CallFunction|ResetGravity)
  (if (AI|Components|NavMovement|IsMovingonGround (Variables|Character|GetCharacterMovement))
    (Variables|Default|SetCurrentState "NewEnumerator0")
    (else
      (Variables|Default|SetCurrentState "NewEnumerator8"))))

(fn SetWallClinging
  (params (bWallClinging :type Boolean))
  (bind _charactermovement (Variables|Character|GetCharacterMovement))
  (bind _charactermovement_2 (Variables|Character|GetCharacterMovement))
  (if bWallClinging
    (Variables|Default|SetCurrentState "NewEnumerator11")
    (Variables|/Script/Engine.MovementComponent|SetVelocity _charactermovement "0, 0, 0")
    (Pawn|Components|CharacterMovement|SetMovementMode _charactermovement "MOVE_Flying" 0)
    (elif (AI|Components|NavMovement|IsMovingonGround (Variables|Character|GetCharacterMovement))
      (Variables|Default|SetCurrentState "NewEnumerator0")
      (Pawn|Components|CharacterMovement|SetMovementMode _charactermovement_2 "MOVE_Walking" 0)
      (else
        (Variables|Default|SetCurrentState "NewEnumerator8")
        (Pawn|Components|CharacterMovement|SetMovementMode _charactermovement_2 "MOVE_Falling" 0))))
  (CallFunction|UpdateAnimation))