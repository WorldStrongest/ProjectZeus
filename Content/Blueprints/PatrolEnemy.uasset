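; PatrolEnemy is an enemy that walks back and forth along the world X axis between two endpoints.
; On BeginPlay it converts the left and right endpoint offsets into world positions relative to its spawn location.
; Each Tick it adds movement input in the current direction and flips the MovingRight flag once its X position passes the endpoint it is heading toward.
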(event EventBeginPlay
  ;[1 1 1] BeginPlay
  (Variables|Default|SetRightEndPoint (+ (Transformation|GetActorLocation) (Variables|Default|GetRightEndPoint)))
  (Variables|Default|SetLeftEndPoint (+ (Transformation|GetActorLocation) (Variables|Default|GetLeftEndPoint))))

(event Collision|EventActorBeginOverlap
  (params (OtherActor :type Actor%20Object%20Reference)))

(event EventTick
  (params (DeltaSeconds :type Float%20%28single-precision%29))
  (bind _returnvalue (Transformation|GetActorLocation))
  (bind _x (Math|Vector|BreakVector _returnvalue))
  ;[1 1 1] Tick
  (Pawn|Input|AddMovementInput (Math|Vector|SelectVector "1.000000, 0, 0" "-1.000000, 0, 0" (Variables|Default|GetMovingRight)) 1.0 false)
  (if (Variables|Default|GetMovingRight)
    (if (>= _x (.X (Math|Vector|BreakVector (Variables|Default|GetRightEndPoint))))
      (Variables|Default|SetMovingRight false))
    (elif (<= _x (.X (Math|Vector|BreakVector (Variables|Default|GetLeftEndPoint))))
      (Variables|Default|SetMovingRight true))))

(fn ConstructionScript)