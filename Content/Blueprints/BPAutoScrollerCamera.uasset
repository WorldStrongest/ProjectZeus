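; Auto-scroller camera actor that moves along world X independently of the player.
; On BeginPlay it snaps to the player pawn's X and Z at a set Y, then adds CameraSpeed along X every tick, unscaled by delta time.
; Each tick it also projects the pawn to screen space and prints whether it is past a margin beyond the left edge, with no other consequence.
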(event EventBeginPlay
  (bind _returnvalue (Game|Player|GetPlayerPawn 0))
  (bind _returnvalue_2 (Transformation|GetActorLocation _returnvalue))
  (bind (_x _y _z) (Math|Vector|BreakVector _returnvalue_2))
  (Transformation|SetActorLocation (Math|Vector|MakeVector _x (Variables|Default|GetYLocation) _z) false false))

(event Collision|EventActorBeginOverlap
  (params (OtherActor :type Actor%20Object%20Reference)))

(event EventTick
  (params (DeltaSeconds :type Float%20%28single-precision%29))
  (Transformation|AddActorWorldOffset (Math|Vector|MakeVector (Variables|Default|GetCameraSpeed) 0.0 0.0))
  (if (<= (.X (Math|Vector2D|BreakVector2D (.ScreenPosition (Class|GameplayStatics|ProjectWorldtoScreen (Game|GetPlayerController 0) (Transformation|GetActorLocation (Game|Player|GetPlayerPawn 0)) false)))) -5e+01)
    (Development|PrintString "True")
    (else
      (Development|PrintString "False"))))

(fn ConstructionScript)