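; BPLadder is a climbable 2D ladder actor that builds itself to the height between LadderBottom and LadderTop.
; The construction script stacks non-colliding Paper2D sprites every RungOffset, cycling through LadderPartSprite and skipping index 0 on wrap.
; It sizes and centers a thin trigger Box from the rung count, using a hardcoded half-spacing.
; Box overlap sets Climbable on BPPlayer, and end overlap calls SetNotClimbing.
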(event OnComponentBeginOverlap(Box)
  (params (OverlappedComponent :type Primitive%20Component%20Object%20Reference) (OtherActor :type Actor%20Object%20Reference) (OtherComp :type Primitive%20Component%20Object%20Reference) (OtherBodyIndex :type Integer) (bFromSweep :type Boolean) (SweepResult :type Hit%20Result%20Structure%20%28by%20ref%29))
  (bind _asbpplayer (Utilities|Casting|CastToBPPlayer OtherActor))
  (Variables|/Game/Blueprints/BPPlayer.BPPlayer_C|SetbClimbable _asbpplayer true))

(event OnComponentEndOverlap(Box)
  (params (OverlappedComponent :type Primitive%20Component%20Object%20Reference) (OtherActor :type Actor%20Object%20Reference) (OtherComp :type Primitive%20Component%20Object%20Reference) (OtherBodyIndex :type Integer))
  (bind _asbpplayer (Utilities|Casting|CastToBPPlayer OtherActor))
  (Default|SetNotClimbing _asbpplayer))

(event EventBeginPlay)

(event Collision|EventActorBeginOverlap
  (params (OtherActor :type Actor%20Object%20Reference)))

(event EventTick
  (params (DeltaSeconds :type Float%20%28single-precision%29)))

(fn ConstructionScript
  (bind _laddertop (Variables|Default|GetLadderTop))
  (bind _ladderbottom (Variables|Default|GetLadderBottom))
  (bind _rungoffset (Variables|Default|GetRungOffset))
  (bind _box (Variables|Default|GetBox))
  (bind _returnvalue (- _laddertop _ladderbottom))
  (bind _z (Math|Vector|BreakVector _returnvalue))
  (bind _returnvalue_2 (/ _z _rungoffset))
  (bind _returnvalue_3 (Math|Float|Truncate _returnvalue_2))
  (Utilities|FlowControl|Sequence
    (:then_0
      (for _index (range 0 _returnvalue_3)
        (bind _returnvalue_4 (AddComponent|AddPaperSpriteComponent false (Math|Transform|MakeTransform (Math|Transform|TransformLocation (Math|Transform|MakeTransform "0, 0, 0") (Math|Vector|MakeVector 0.0 0.0 (* _index _rungoffset))))))
        (Rendering|Components|Sprite|SetSprite _returnvalue_4 (Utilities|Array|Get(acopy) (Variables|Default|GetLadderPartSprite) (Variables|Default|GetSpriteIndex)))
        (bind _result (Math|Integer|IncrementInt (Variables|Default|GetSpriteIndex))
          (:%20%20
            (bind _output_get (Variables|Default|SetSpriteIndex (Math|Integer|%(Integer) _result (Utilities|Array|Length (Variables|Default|GetLadderPartSprite)))))
            (if (== _output_get 0)
              (Math|Integer|IncrementInt (Variables|Default|GetSpriteIndex)
                (:%20%20
                  _)))
            (Collision|SetCollisionEnabled _returnvalue_4 "NoCollision"))))
      (Components|Box|SetBoxExtent _box (Math|Vector|MakeVector 1.0 1.0 (* _returnvalue_3 8.0)) true)
      (Transformation|SetRelativeLocation _box (Math|Vector|MakeVector 0.0 0.0 (* _returnvalue_3 8.0)) false false))))