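; Beta follow camera that tracks the player on X and Z while keeping its own Y, as in a side-scroller.
; It snaps to the player on BeginPlay, then on Tick eases its SceneComponent toward them with MoveComponentTo whenever HorizFollowBox has no overlaps.
; Height follows only if VertFollowBox is also empty.
; Left/right box overlaps are empty; the camera X-shift logic is disconnected, and CameraXOffset is stored but unused.
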(event OnComponentBeginOverlap(RightBox)
  (params (OverlappedComponent :type Primitive%20Component%20Object%20Reference) (OtherActor :type Actor%20Object%20Reference) (OtherComp :type Primitive%20Component%20Object%20Reference) (OtherBodyIndex :type Integer) (bFromSweep :type Boolean) (SweepResult :type Hit%20Result%20Structure%20%28by%20ref%29)))

(event OnComponentBeginOverlap(LeftBox)
  (params (OverlappedComponent :type Primitive%20Component%20Object%20Reference) (OtherActor :type Actor%20Object%20Reference) (OtherComp :type Primitive%20Component%20Object%20Reference) (OtherBodyIndex :type Integer) (bFromSweep :type Boolean) (SweepResult :type Hit%20Result%20Structure%20%28by%20ref%29)))

(event EventBeginPlay
  (bind _returnvalue (Game|Player|GetPlayerPawn 0))
  (bind _returnvalue_2 (Transformation|GetActorLocation _returnvalue))
  (bind (_x _y _z) (Math|Vector|BreakVector _returnvalue_2))
  (Transformation|SetActorLocation (Math|Vector|MakeVector _x (.Y (Math|Vector|BreakVector (Transformation|GetActorLocation))) _z) false false)
  (Variables|Default|SetCameraXOffset (* (.X (Math|Vector|BreakVector (Variables|/Script/Engine.SceneComponent|GetRelativeLocation (Variables|CameraActor|GetCameraComponent)))) -1.0)))

(event EventTick
  (params (DeltaSeconds :type Float%20%28single-precision%29))
  (bind _returnvalue (Game|Player|GetPlayerPawn 0))
  (bind _returnvalue_2 (Transformation|GetActorTransform))
  (bind _returnvalue_3 (Transformation|GetActorTransform _returnvalue))
  (bind _location (Math|Transform|BreakTransform _returnvalue_2))
  (bind _location_2 (Math|Transform|BreakTransform _returnvalue_3))
  (bind (_x _y _z) (Math|Vector|BreakVector _location))
  (bind (_x_2 _y_2 _z_2) (Math|Vector|BreakVector _location_2))
  (if (== (Utilities|Array|Length (Class|PrimitiveComponent|GetOverlappingComponents (Variables|Default|GetHorizFollowBox))) 0)
    (Utilities|IsValid (Game|Player|GetPlayerPawn 0)
      (:Is%20Valid
        (Components|MoveComponentTo (Variables|Default|GetSceneComponent) (Math|Vector|MakeVector _x_2 _y (Math|Float|SelectFloat _z_2 _z (== (Utilities|Array|Length (Class|PrimitiveComponent|GetOverlappingComponents (Variables|Default|GetVertFollowBox))) 0))) "0, 0, 0" false false 0.6 false)))))

(fn ConstructionScript)